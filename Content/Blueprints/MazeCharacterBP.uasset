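; Player character for a maze game, with pickups, an enemy stun ability and game-state screens.
; Overlaps route by cast to health, timed speed boost, damage or victory, with any other actor triggering a stun trace.
; The Stun input sphere-traces to stun NPCEnemyBP actors, on a cooldown counted down in Tick.
; It creates the HUD, toggles pause, and hard-codes keys for game over, self-damage and temporarily hiding the stun UI.
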(event EventBeginPlay
  (bind _returnvalue (UserInterface|CreateWidget "/Game/Blueprints/Widgets/PlayerUI.PlayerUI_C"))
  (UserInterface|Viewport|AddtoViewport _returnvalue 0)
  (bind _returnvalue_2 (UserInterface|CreateWidget "/Game/Blueprints/Widgets/StunUI.StunUI_C"))
  (UserInterface|Viewport|AddtoViewport _returnvalue_2 0))

(event Collision|EventActorBeginOverlap
  (params (OtherActor :type Actor%20Object%20Reference))
  (bind _returnvalue (Transformation|GetActorLocation))
  (Utilities|Casting|CastToBP_HealthPickup OtherActor
    (:then
      (Class|MazeCharacter|TakeDamage -1e+01 (Variables|Default|GetDamage%20Event)))
    (:CastFailed
      (Utilities|Casting|CastToBP_SpeedPickup OtherActor
        (:then
          (Variables|/Script/Engine.CharacterMovementComponent|SetMaxWalkSpeed (Variables|Character|GetCharacterMovement) 9e+02)
          (Utilities|FlowControl|Delay 5.0)
          (Variables|/Script/Engine.CharacterMovementComponent|SetMaxWalkSpeed (Variables|Character|GetCharacterMovement) 6e+02))
        (:CastFailed
          (Utilities|Casting|CastToDamage_Pickup OtherActor
            (:then
              (Class|MazeCharacter|TakeDamage 1e+02 (Variables|Default|GetDamage%20Event))
              (Effects|SpawnEmitteratLocation "/Game/Realistic_Starter_VFX_Pack_Vol2/Particles/Blood/P_Blood_Splat_Cone.P_Blood_Splat_Cone" (Transformation|GetActorLocation)))
            (:CastFailed
              (Utilities|Casting|CastToBP_VictoryItem OtherActor
                (:then
                  (bind _returnvalue_2 (UserInterface|CreateWidget "/Game/Blueprints/Widgets/VictoryWidgetBP.VictoryWidgetBP_C"))
                  (UserInterface|Viewport|AddtoViewport _returnvalue_2 0)
                  (Variables|/Script/Engine.PlayerController|SetbShowMouseCursor (Game|GetPlayerController 0) true)
                  (Game|SetGamePaused true))
                (:CastFailed
                  (bind _outhits (Collision|MultiSphereTraceForObjects _returnvalue _returnvalue (Variables|Default|GetGlobal%20Stun%20Radius) (Variables|Default|GetStun%20Trace%20Types) false 0 "None"))
                  (for _array_element _outhits
                    (bind _asnpcenemy_bp (Utilities|Casting|CastToNPCEnemyBP (.HitActor (Collision|BreakHitResult _array_element))))
                    (Default|Stunned _asnpcenemy_bp)))))))))))

(event EventTick
  (params (DeltaSeconds :type Float%20%28single-precision%29))
  (if (> (Variables|Default|GetStunCooldown) 0.0)
    (Variables|Default|SetStunCooldown (- (Variables|Default|GetStunCooldown) DeltaSeconds))))

(event Input|ActionEvents|InputActionStun
  (params (Key :type Key%20Structure :default "None"))
  (bind _returnvalue (Transformation|GetActorLocation))
  ;[1 1 1] Stun System
  (:Pressed
    (if (<= (Variables|Default|GetStunCooldown) 0.0)
      (Variables|Default|SetStunCooldown (Variables|Default|GetTimeBetweenStuns))
      (Class|MazeCharacter|ActivateStunParticleSystem)
      (bind _outhits (Collision|MultiSphereTraceForObjects _returnvalue _returnvalue (Variables|Default|GetStunTraceRaidus) (Variables|Default|GetStun%20Trace%20Types) false 0 "None"))
      (for _array_element _outhits
        (bind _asnpcenemy_bp (Utilities|Casting|CastToNPCEnemyBP (.HitActor (Collision|BreakHitResult _array_element))))
        (Default|Stunned _asnpcenemy_bp)))))

(event Input|KeyboardEvents|K
  (params (Key :type Key%20Structure :default "None"))
  (:Pressed
    (bind _returnvalue (UserInterface|CreateWidget "/Game/Blueprints/Widgets/GameOverWidgetBP.GameOverWidgetBP_C"))
    (UserInterface|Viewport|AddtoViewport _returnvalue 0)
    (Variables|/Script/Engine.PlayerController|SetbShowMouseCursor (Game|GetPlayerController 0) true)
    (Game|SetGamePaused true)))

(event Input|KeyboardEvents|1
  (params (Key :type Key%20Structure :default "None"))
  (:Pressed
    (bind _returnvalue (Game|Damage|ApplyDamage self 1e+01 0 0))
    (Variables|Default|SetHealth (Math|Float|Clamp(Float) (- (Variables|Default|GetHealth) _returnvalue) 0.0 (Variables|Default|GetMax%20Health)))))

(event Input|KeyboardEvents|R
  (params (Key :type Key%20Structure :default "None"))
  (bind _returnvalue (Game|GetPlayerController 0))
  ;[1 1 1] Pauses the game
  (:Pressed
    (if (not (Variables|Default|GetIsPaused?))
      (Variables|Default|SetIsPaused? true)
      (bind _returnvalue_2 (UserInterface|CreateWidget "/Game/Blueprints/Widgets/PauseMenuBP.PauseMenuBP_C" _returnvalue))
      (bind _output_get (Variables|Default|SetPauseMenuWidget _returnvalue_2))
      (UserInterface|Viewport|AddtoViewport _output_get 0)
      (Input|SetInputModeGameandUI _returnvalue (Variables|Default|GetPauseMenuWidget) "DoNotLock" true)
      (Variables|/Script/Engine.PlayerController|SetbShowMouseCursor (Game|GetPlayerController 0) true)
      (Game|SetGamePaused true)
      (else
        (Variables|Default|SetIsPaused? false)
        (Widget|RemovefromParent (Variables|Default|GetPauseMenuWidget))
        (Game|SetGamePaused false)
        (Input|SetInputModeGameOnly _returnvalue)
        (Variables|/Script/Engine.PlayerController|SetbShowMouseCursor (Game|GetPlayerController 0) true)))))

(event Input|KeyboardEvents|SpaceBar
  (params (Key :type Key%20Structure :default "None"))
  (:Pressed
    (bind _foundwidgets (Widget|GetAllWidgetsOfClass "/Game/Blueprints/Widgets/StunUI.StunUI_C" true))
    (Widget|RemovefromParent _foundwidgets)
    (Utilities|FlowControl|Delay 3.0)
    (bind _returnvalue (UserInterface|CreateWidget "/Game/Blueprints/Widgets/StunUI.StunUI_C"))
    (UserInterface|Viewport|AddtoViewport _returnvalue 0)))

(fn ConstructionScript)